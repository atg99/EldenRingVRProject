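; BP_TEnemyAIController is an enemy AI controller that reacts to sounds picked up by its AiPercep perception component.
; On each perception update it resolves the stimulus's sense class and, for hearing, checks whether the source actor is tagged Player or Enemy.
; Each case only prints a debug string; other senses are ignored, and BeginPlay, Tick and the construction script are empty.
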(event `self.ReceiveBeginPlay`)

(event `self.ReceiveTick`
  (params (DeltaSeconds :type "Float (single-precision)")))

(event `self.aiPercep.OnTargetPerceptionUpdated`
  (params (Actor :type "Actor Object Reference") (Stimulus :type "AIStimulus Structure"))
  (bind _returnvalue (`AIPerceptionSystem.GetSenseClassForStimulus` Stimulus))
  (bind _returnvalue_2 (== _returnvalue "/Script/AIModule.AISense_Hearing"))
  (if (and _returnvalue_2 (`self.ActorHasTag` Actor "Player"))
    (`KismetSystemLibrary.PrintString` "HearingPlayer")
    (elif (and _returnvalue_2 (`self.ActorHasTag` Actor "Enemy"))
      (`KismetSystemLibrary.PrintString` "HearingEnemy"))))

(fn `UserConstructionScript`)