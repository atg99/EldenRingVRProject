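; Dismemberment actor that severs a given bone on its skeletal mesh and leaves blood on the surface below.
; Desmemberment breaks the bone's constraint, then enables physics for lower-spine and leg bones, or spawns separate head/body actors and hides the bone for Head and Spine 02.
; It applies an impulse and traces downward to place a blood decal.
; CalculateImpulse's camera-based math is unconnected, and the EventGraph's all-socket loop never runs.
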(event `self.ReceiveBeginPlay`)

(fn `Desmemberment`
  (params (Bone :type Name))
  (bind _skeletalmesh (`self.SkeletalMesh`))
  (bind _skeletalmesh_2 (`self.SkeletalMesh`))
  (bind _array_element_0 (`self.Array Element_0`))
  (bind _returnvalue (`SceneComponent.GetSocketLocation` _skeletalmesh_2 _array_element_0))
  (bind _returnvalue_2 (`SceneComponent.GetSocketTransform` (`self.SkeletalMesh`) (`self.Array Element_0`) "RTS_World"))
  (`KismetSystemLibrary.PrintString` (`KismetStringLibrary.Conv_NameToString` Bone))
  (bind _output_get (set `self.Array Element_0` Bone))
  (`SkeletalMeshComponent.BreakConstraint` (`self.SkeletalMesh`) (0.0 0.0 0.0) (0.0 0.0 0.0) _output_get)
  (switch `name` _output_get
    (:`Default`
      _)
    (:`spine_01`
      (`PrimitiveComponent.SetSimulatePhysics` _skeletalmesh true :!label _label)
      (`PrimitiveComponent.AddImpulseAtLocation` _skeletalmesh (`self.CalculateImpulse`) (`SceneComponent.GetSocketLocation` _skeletalmesh_2 _array_element_0) _array_element_0 :!label _label_2))
    (:`thigh_l`
      (goto _label))
    (:`thigh_r`
      (goto _label))
    (:`calf_l`
      (goto _label))
    (:`calf_r`
      (goto _label))
    (:`foot_l`
      (goto _label))
    (:`foot_r`
      (goto _label))
    (:`head`
      (`|SpawnActorFromClass` "/Game/Geometrys/BP_ManneyHead.BP_ManneyHead_C" _returnvalue_2 "Undefined" "OverrideRootScale" null null)
      (`SkinnedMeshComponent.HideBoneByName` (`self.SkeletalMesh`) (`self.Array Element_0`) "PBO_None" :!label _label_3)
      (goto _label_2))
    (:`spine_02`
      (`|SpawnActorFromClass` "/Game/Geometrys/BP_ManneyBoby.BP_ManneyBoby_C" _returnvalue_2 "Undefined" "OverrideRootScale" null null)
      (goto _label_3)))
  (bind _outhit (`KismetSystemLibrary.LineTraceSingle` _returnvalue (+ _returnvalue (* (0.0 0.0 -1.0) (0.0 0.0 1500.0))) "TraceTypeQuery1"))
  (bind (_bblockinghit _binitialoverlap _time _distance _location _impactpoint _normal) (`GameplayStatics.BreakHitResult` _outhit))
  (`GameplayStatics.SpawnDecalAtLocation` "/Game/Megascans/Decals/High_Velocity_Blood_Spatter_sfhuaivp/MI_High_Velocity_Blood_Spatter_sfhuaivp_2K.MI_High_Velocity_Blood_Spatter_sfhuaivp_2K" (-63.0 -128.0 -128.0) _location (`KismetMathLibrary.Conv_VectorToRotator` _normal) 60.0))

(fn `UserConstructionScript`)