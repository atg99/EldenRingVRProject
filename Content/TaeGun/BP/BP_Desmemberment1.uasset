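; Dismemberment test actor that breaks a skeletal mesh apart at a given bone and can blend it back together.
; Desmemberment breaks the constraint, simulates physics on torso and leg bones, and traces down for a blood decal.
; Its hide event swaps head or spine_02 for spawned pieces with a brief field burst.
; Merging copies the pose to a PoseableMesh, which Tick lerps toward Origin; the transform-recording rewind is disconnected.
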(event `self.ReceiveBeginPlay`)

(event `self.ReceiveTick`
  (params (DeltaSeconds :type "Float (single-precision)"))
  (bind _poseablemesh (`self.PoseableMesh`))
  (if (`self.bStartReverse`)
    (bind _output_get (set `self.Timer` (+ DeltaSeconds (`self.Timer`))))
    (`KismetSystemLibrary.PrintString` (`KismetStringLibrary.Conv_DoubleToString` _output_get))
    (bind _output_get_2 (set `self.Time` (+ (* DeltaSeconds 0.01) (`self.Time`))))
    (for (_array_element _array_index) (`SceneComponent.GetAllSocketNames` _poseablemesh)
      (`PoseableMeshComponent.SetBoneTransformByName` _poseablemesh _array_element (`KismetMathLibrary.TLerp` (`SceneComponent.GetSocketTransform` _poseablemesh _array_element "RTS_World") (`SceneComponent.GetSocketTransform` (`self.Origin`) (`|GetArrayItem` (`SceneComponent.GetAllSocketNames` (`self.Origin`)) _array_index) "RTS_World") _output_get_2) "WorldSpace"))))

(event `hide`
  (params (bone :type Name))
  (bind _bone (`self.Bone`))
  (bind _returnvalue (`SceneComponent.GetSocketTransform` (`self.SkeletalMesh`) _bone "RTS_World"))
  (bind _output_get (set `self.Bone` bone))
  (`KismetSystemLibrary.PrintString` (`KismetStringLibrary.Conv_NameToString` _output_get))
  (switch `name` _bone
    (:`head`
      (`KismetSystemLibrary.PrintString` "hide")
      (`|SpawnActorFromClass` "/Game/Geometrys/BP_ManneyHead.BP_ManneyHead_C" _returnvalue "Undefined" "OverrideRootScale" null null))
    (:`spine_02`
      (`|SpawnActorFromClass` "/Game/Geometrys/BP_ManneyBoby.BP_ManneyBoby_C" _returnvalue "Undefined" "OverrideRootScale" null null)))
  (`SkinnedMeshComponent.HideBoneByName` (`self.SkeletalMesh`) _bone "PBO_None")
  (bind _returnvalue_2 (`|SpawnActorFromClass` "/Engine/EditorResources/FieldNodes/FS_MasterField.FS_MasterField_C" _returnvalue "Undefined" "OverrideRootScale" null null))
  (`KismetSystemLibrary.PrintString` "Hello")
  (set `/Engine/EditorResources/FieldNodes/FS_MasterField.ActivationType` "NewEnumerator4" _returnvalue_2)
  (`/Engine/EditorResources/FieldNodes/FS_MasterField.CE_Trigger` _returnvalue_2)
  (`KismetSystemLibrary.Delay` 0.2)
  (`self.K2_DestroyActor` _returnvalue_2))

(fn `Desmemberment`
  (params (Bone :type Name))
  (bind _array_element_0 (`self.Array Element_0`))
  (bind _skeletalmesh (`self.SkeletalMesh`))
  (bind _skeletalmesh_2 (`self.SkeletalMesh`))
  (bind _returnvalue (`SceneComponent.GetSocketLocation` _skeletalmesh_2 _array_element_0))
  (`BlueprintSetLibrary.Set_Add` (`self.Bones`) Bone)
  (`KismetSystemLibrary.PrintString` (`KismetStringLibrary.Conv_NameToString` Bone))
  (bind _output_get (set `self.Array Element_0` Bone))
  (`SkeletalMeshComponent.BreakConstraint` (`self.SkeletalMesh`) (0.0 0.0 0.0) (0.0 0.0 0.0) _output_get)
  (switch `name` _output_get
    (:`Default`
      _)
    (:`spine_01`
      (`PrimitiveComponent.SetSimulatePhysics` _skeletalmesh true :!label _label)
      (`PrimitiveComponent.AddImpulseAtLocation` _skeletalmesh (`self.CalculateImpulse`) (`SceneComponent.GetSocketLocation` _skeletalmesh_2 _array_element_0) _array_element_0))
    (:`thigh_l`
      (goto _label))
    (:`thigh_r`
      (goto _label))
    (:`calf_l`
      (goto _label))
    (:`calf_r`
      (goto _label))
    (:`foot_l`
      (goto _label))
    (:`foot_r`
      (goto _label)))
  (bind _outhit (`KismetSystemLibrary.LineTraceSingle` _returnvalue (+ _returnvalue (* (0.0 0.0 -1.0) (0.0 0.0 1500.0))) "TraceTypeQuery1"))
  (bind (_bblockinghit _binitialoverlap _time _distance _location _impactpoint _normal) (`GameplayStatics.BreakHitResult` _outhit))
  (`GameplayStatics.SpawnDecalAtLocation` "/Game/Megascans/Decals/High_Velocity_Blood_Spatter_sfhuaivp/MI_High_Velocity_Blood_Spatter_sfhuaivp_2K.MI_High_Velocity_Blood_Spatter_sfhuaivp_2K" (-63.0 -128.0 -128.0) _location (`KismetMathLibrary.Conv_VectorToRotator` _normal) 60.0)
  (`self.hide` (`self.Array Element_0`))
  (set `self.bStartRecoding` true))

(fn `merging`
  (bind _poseablemesh (`self.PoseableMesh`))
  (bind _skeletalmesh (`self.SkeletalMesh`))
  (for (_array_element _array_index) (`SceneComponent.GetAllSocketNames` _poseablemesh)
    (`PoseableMeshComponent.SetBoneTransformByName` _poseablemesh _array_element (`SceneComponent.GetSocketTransform` _skeletalmesh (`|GetArrayItem` (`SceneComponent.GetAllSocketNames` _skeletalmesh) _array_index) "RTS_World") "WorldSpace"))
  (set `SkeletalMeshComponent.bPauseAnims` true (`self.SkeletalMesh`))
  (set `self.bStartReverse` true)
  (`KismetSystemLibrary.PrintString` "reverse1"))

(fn `UserConstructionScript`)