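; BP_Chains is a physics-chain VR hazard with a sausage mesh that damages the player and can be destroyed by sword.
; While alive, a sphere overlap flings Chain8 toward the player.
; Sword overlaps on the sausage subtract swing speed from HP.
; At zero, constraints break, links ragdoll, and a procedural copy of the sausage, built in construction, replaces it, sliced by sword direction with capped faces and a Niagara blood burst.
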(event `self.ReceiveBeginPlay`
  (set `self.HP` 100.0))

(event `self.Sphere.OnComponentBeginOverlap`
  (params (OverlappedComponent :type "PrimitiveComponent Object Reference") (OtherActor :type "Actor Object Reference") (OtherComp :type "PrimitiveComponent Object Reference") (OtherBodyIndex :type Integer) (bFromSweep :type Boolean) (SweepResult :type "HitResult Structure (by ref)"))
  (bind _chain8 (`self.chain8`))
  (bind _asbp_vrplayer (cast `/Game/UyYeon/Blueprint/BP_VRPlayer` OtherActor))
  (if (> (`self.HP`) 0.0)
    (`PrimitiveComponent.AddImpulse` _chain8 (* (`KismetMathLibrary.Normal` (- (`self.K2_GetActorLocation` _asbp_vrplayer) (`SceneComponent.K2_GetComponentLocation` _chain8))) 600.0) "None" true)))

(event `self.Sausage.OnComponentBeginOverlap`
  (params (OverlappedComponent :type "PrimitiveComponent Object Reference") (OtherActor :type "Actor Object Reference") (OtherComp :type "PrimitiveComponent Object Reference") (OtherBodyIndex :type Integer) (bFromSweep :type Boolean) (SweepResult :type "HitResult Structure (by ref)"))
  (bind _proceduralmesh (`self.ProceduralMesh`))
  (bind _returnvalue (`SceneComponent.K2_GetComponentLocation` _proceduralmesh))
  (bind _asbp_vrplayer (cast `/Game/UyYeon/Blueprint/BP_VRPlayer` OtherActor)
    (:`then`
      (`VRPlayer.OnDamaged` _asbp_vrplayer 10.0)
      (`KismetSystemLibrary.PrintString` "d"))
    (:`CastFailed`
      _))
  (bind _asbp_psword_1 (cast `/Game/UyYeon/Blueprint/BP_PSword1` OtherActor))
  (bind _returnvalue_2 (`PlayerWeapon.GetSwordSpeedfloat` _asbp_psword_1))
  (`KismetSystemLibrary.PrintString` (`KismetStringLibrary.Conv_DoubleToString` _returnvalue_2))
  (bind _output_get (set `self.HP` (- (`self.HP`) _returnvalue_2)))
  (`KismetSystemLibrary.PrintString` (`KismetStringLibrary.Conv_DoubleToString` _output_get))
  (if (<= (`self.HP`) 0.0)
    (`PhysicsConstraintComponent.BreakConstraint` (`self.PhysicsConstraint`))
    (`PhysicsConstraintComponent.BreakConstraint` (`self.PhysicsConstraint1`))
    (`PhysicsConstraintComponent.BreakConstraint` (`self.PhysicsConstraint2`))
    (`PhysicsConstraintComponent.BreakConstraint` (`self.PhysicsConstraint3`))
    (`PhysicsConstraintComponent.BreakConstraint` (`self.PhysicsConstraint6`))
    (`PhysicsConstraintComponent.BreakConstraint` (`self.PhysicsConstraint4`))
    (`PhysicsConstraintComponent.BreakConstraint` (`self.PhysicsConstraint5`))
    (`PhysicsConstraintComponent.BreakConstraint` (`self.PhysicsConstraint7`))
    (`PrimitiveComponent.SetCollisionProfileName` (`self.chain4`) "Ragdoll" false)
    (`PrimitiveComponent.SetCollisionProfileName` (`self.chain7`) "Ragdoll" false)
    (`PrimitiveComponent.SetCollisionProfileName` (`self.chain6`) "Ragdoll" false)
    (`PrimitiveComponent.SetCollisionProfileName` (`self.chain1`) "Ragdoll" false)
    (`PrimitiveComponent.SetCollisionProfileName` (`self.chain2`) "Ragdoll" false)
    (`PrimitiveComponent.SetCollisionProfileName` (`self.chain5`) "Ragdoll" false)
    (`PrimitiveComponent.SetCollisionProfileName` (`self.chain3`) "Ragdoll" false)
    (`PrimitiveComponent.SetCollisionProfileName` (`self.chain8`) "Ragdoll" false)
    (`SceneComponent.SetVisibility` _proceduralmesh true false)
    (`PrimitiveComponent.SetCollisionProfileName` _proceduralmesh "Ragdoll" true)
    (`PrimitiveComponent.SetSimulatePhysics` _proceduralmesh true)
    (`KismetProceduralMeshLibrary.SliceProceduralMesh` _proceduralmesh _returnvalue (`KismetMathLibrary.Normal` (- _returnvalue (`SceneComponent.K2_GetComponentLocation` (`PlayerWeapon.meshComp` _asbp_psword_1)))) true "CreateNewSectionForCap" "/Game/TaeGun/Material/M_BloodMat_Inst.M_BloodMat_Inst")
    (`NiagaraFunctionLibrary.SpawnSystemAtLocation` "/Game/BloodPack/Burst/Niagara/NS_BloodBurst_Med.NS_BloodBurst_Med" _returnvalue)
    (`SceneComponent.SetVisibility` (`self.Sausage`) false false)))

(event `self.Sausage.OnComponentHit`
  (params (HitComponent :type "PrimitiveComponent Object Reference") (OtherActor :type "Actor Object Reference") (OtherComp :type "PrimitiveComponent Object Reference") (NormalImpulse :type "Vector Structure") (Hit :type "HitResult Structure (by ref)")))

(fn `UserConstructionScript`
  (`KismetProceduralMeshLibrary.CopyProceduralMeshFromStaticMeshComponent` (`self.Sausage`) 0 (`self.ProceduralMesh`) true))