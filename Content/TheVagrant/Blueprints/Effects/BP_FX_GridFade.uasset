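; BP_FX_GridFade is an effect Blueprint built on a Plane component, named for a grid fade whose look comes from its material.
; Its construction script creates a dynamic material instance on the plane from SourceMaterial.
; It then copies the Color, A, B and Percent variables into the matching material parameters, with no runtime animation in the graph shown.
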(fn `UserConstructionScript`
  (bind _returnvalue (`PrimitiveComponent.CreateDynamicMaterialInstance` (`self.Plane`) 0 (`self.Source Material`) "None"))
  (`MaterialInstanceDynamic.SetVectorParameterValue` _returnvalue "Color" (`self.Color`))
  (`MaterialInstanceDynamic.SetScalarParameterValue` _returnvalue "A" (`self.A`))
  (`MaterialInstanceDynamic.SetScalarParameterValue` _returnvalue "B" (`self.B`))
  (`MaterialInstanceDynamic.SetScalarParameterValue` _returnvalue "Percent" (`self.Percent`)))